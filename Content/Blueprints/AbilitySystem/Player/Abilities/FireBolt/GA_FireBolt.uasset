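; Fire Bolt gameplay ability for the player that casts a projectile toward the point under the cursor.
; After committing, a custom target-data task supplies the cursor hit location, which updates the avatar's motion warping facing.
; It plays the cast montage, and a montage gameplay event triggers the projectile spawn from a socket, plus a debug sphere at the target.
; The ability ends on commit failure or when the montage completes, is interrupted or is cancelled.
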(event `self.K2_ActivateAbility`
  (bind _locationundercursor (`self.LocationUnderCursor`))
  (bind _returnvalue (`self.K2_CommitAbility`))
  (if _returnvalue
    ;[0.15 0.15 0.15 0.5 14] С помощью созданного нами AbilityTask_GetTargetDataUnderCursor мы получим координаты нажатия курсором и отправим делегатом сюда
    (bind (_asynctaskproxy _targetdata) (`TargetDataUnderCursor.CreateTargetDataUnderMouse`)
      (:`TargetDataCursorTrace`
        (bind _output_get (set `self.LocationUnderCursor` (`.ImpactPoint` (`GameplayStatics.BreakHitResult` (`AbilitySystemBlueprintLibrary.GetHitResultFromTargetData` _targetdata)))))
        ;[0.15 0.15 0.15 0.5 14] Обновим ориентацию для персонажа
        (message `CombatInterface.UpdateMotionWarping` (`self.GetAvatarActorFromActorInfo`) _output_get)
        (`AbilityTask_PlayMontageAndWait.CreatePlayMontageAndWaitProxy` "None" "/Game/Assets/Characters/Aura/Animations/Abilities/AM_FireBolt.AM_FireBolt" 1.0 "None" true 1.0 0.0 true
          (:`then`
            (`AbilityTask_WaitGameplayEvent.WaitGameplayEvent` (struct :`TagName` "Event.MontageTag.FireBolt") null true
              (:`EventReceived`
                (`self.SpawnProjectile` _locationundercursor (`self.Socket Tag`))
                (`KismetSystemLibrary.DrawDebugSphere` _locationundercursor 10.0 12 (struct :`R` 1.0 :`B` 0.005661 :`A` 1.0) 5.0 1.0))))
          (:`OnCompleted`
            (`self.K2_EndAbility` :!label _label))
          (:`OnInterrupted`
            (goto _label))
          (:`OnCancelled`
            (goto _label)))))
    (else
      (`self.K2_EndAbility`))))