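; GA_ListenForEvent is a passive gameplay ability that turns incoming Attribute.Meta gameplay events into effects on its owner.
; On activation it prints the avatar's name, then waits for events under that tag, child tags included.
; Each event builds a level 1 EventBasedEffectClass spec, passing the event's tag and magnitude through as SetByCaller, and applies it to the owner.
; It never calls EndAbility, so it keeps listening.
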(event `self.K2_ActivateAbility`
  (`KismetSystemLibrary.PrintString` (`KismetStringLibrary.Concat_StrStr` "ListenForEvent: " (`KismetSystemLibrary.GetObjectName` (`self.GetAvatarActorFromActorInfo`))) true true (struct :`G` 0.66 :`B` 1.0 :`A` 1.0) 2.0 "124125125")
  (bind (_asynctaskproxy _payload) (`AbilityTask_WaitGameplayEvent.WaitGameplayEvent` (struct :`TagName` "Attribute.Meta") null false false)
    (:`EventReceived`
      (bind (_eventtag _instigator _target _optionalobject _optionalobject2 _contexthandle _instigatortags _targettags _eventmagnitude) (break `GameplayEventData` _payload))
      (bind _returnvalue (`AbilitySystemBlueprintLibrary.AssignTagSetByCallerMagnitude` (`AbilitySystemComponent.MakeOutgoingSpec` :`self` (`self.GetAbilitySystemComponentFromActorInfo`) :`GameplayEffectClass` (`self.Event Based Effect Class`) :`Level` 1.0) _eventtag _eventmagnitude))
      (`self.K2_ApplyGameplayEffectSpecToOwner` _returnvalue))))