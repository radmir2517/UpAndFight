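; Enemy summon ability, cast to the Goblin Shaman, that spawns random minions while facing the blackboard target via motion warping.
; It plays a random tagged attack montage; the montage's gameplay event shuffles spawn locations and fires a spawn-effect cue at each.
; A looping timer then spawns one minion per tick up to the allotted number, incrementing the shaman's minion count.
; The ability ends when the montage completes or is interrupted, or without a target.
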(event `self.K2_ActivateAbility`
  (set `self.AvatarActor` (`self.GetAvatarActorFromActorInfo`))
  (bind _ascharacter (cast `Character` (`BlackboardComponent.GetValueAsObject` (`AIBlueprintHelperLibrary.GetBlackboard` (`self.AvatarActor`)) (`self.Target Key Name`)))
    (:`then`
      (set `self.TargetCharacter` _ascharacter)
      (set `self.TargetLocation` (`Actor.K2_GetActorLocation` _ascharacter))
      (message `CombatInterface.UpdateMotionWarping` (`self.AvatarActor`) (`self.TargetLocation`))
      (bind (_montage _montagetag) (`self.GetAttackMontage`))
      (`AbilityTask_PlayMontageAndWait.CreatePlayMontageAndWaitProxy` "None" _montage
        (:`then`
          (`AbilityTask_WaitGameplayEvent.WaitGameplayEvent` _montagetag null true
            (:`then`
              (bind _asbp_goblin_shaman (cast `/Game/Blueprints/Character/Shaman/BP_Goblin_Shaman` (`self.AvatarActor`)))
              (set `self.BP Goblin Shaman` _asbp_goblin_shaman))
            (:`EventReceived`
              (bind _returnvalue (`self.GetSpawnLocations`))
              (bind _output_get (set `self.SpawnLocations` _returnvalue))
              (`KismetArrayLibrary.Array_Shuffle` _output_get)
              (for _array_element (`self.SpawnLocations`)
                (`self.K2_ExecuteGameplayCueWithParams` (struct :`TagName` "GameplayCue.SpawnEffect") (`AbilitySystemBlueprintLibrary.MakeGameplayCueParameters` 0.0 0.0 (struct) (struct) (struct) (struct) (struct) _array_element (0.0 0.0 0.0) (`self.TargetCharacter`) (`self.AvatarActor`))))
              (bind _returnvalue_2 (`KismetSystemLibrary.K2_SetTimerDelegate` (delegate `SummonEvent`) (`self.SummonTime`) true))
              (set `self.SummonTimer` _returnvalue_2))))
        (:`OnCompleted`
          (`self.SendGameplayEvent` (struct :`TagName` "Event.Ability.Ended") :!label _label)
          (`self.K2_EndAbility`))
        (:`OnInterrupted`
          (goto _label))
        (:`OnCancelled`
          (goto _label))))
    (:`CastFailed`
      (`self.K2_EndAbility`))))

(event `SummonEvent`
  (if (< (`self.CurrentCount`) (`self.DeltaNumMinions`))
    (bind _returnvalue (`|SpawnActorFromClass` (`self.GetRandomMinionClass`) (`KismetMathLibrary.MakeTransform` (`|GetArrayItem` (`self.SpawnLocations`) (`self.CurrentCount`))) "AdjustIfPossibleButAlwaysSpawn" "MultiplyWithRoot" null (`self.BP Goblin Shaman`)))
    (`/Engine/EditorBlueprintResources/StandardMacros.IsValid` _returnvalue
      (:`Is Valid`
        (`/Engine/EditorBlueprintResources/StandardMacros.IncrementInt` (`self.CurrentCount`)
          (:`  `
            (message `CombatInterface.IncreaseMinionsCount` (`self.BP Goblin Shaman`) 1)))))
    (else
      (`KismetSystemLibrary.K2_ClearAndInvalidateTimerHandle` (`self.SummonTimer`)))))

(fn `GetAttackMontage`
  (returns (Montage :type "AnimMontage Object Reference") (MontageTag :type "GameplayTag Structure") (`Impact Sound` :type "SoundBase Object Reference") (`Socket Location Tag` :type "GameplayTag Structure"))
  (locals (AttackMontages :type "TaggedMontage Structure"))
  (bind _returnvalue (message `CombatInterface.GetAttackMontages` (`self.AvatarActor`)))
  (bind _returnvalue_2 (`self.GetRandomTaggedMontageFromArray` _returnvalue))
  (bind _output_get (set `local.AttackMontages` _returnvalue_2))
  (bind (_montage _montagetag _socketlocationtag _impactsound) (break `TaggedMontage` _output_get))
  (if (!= _montagetag (struct))
    (return _montage _montagetag _impactsound _socketlocationtag)
    (else
      (`self.K2_EndAbility`))))

(fn `OnRep_SpawnLocations`)