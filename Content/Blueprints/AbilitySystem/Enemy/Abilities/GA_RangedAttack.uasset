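; Enemy ranged attack Gameplay Ability that fires a projectile at the Character stored in the AI Blackboard, ending if none is found.
; On activation it captures the target's location, updates the avatar's motion warping and plays a random tagged montage from the avatar's attack montages.
; The montage's gameplay event tag times a single projectile spawn at the captured location.
; The ability ends when the montage completes, is interrupted or is cancelled.
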(event `self.K2_ActivateAbility`
  (set `self.AvatarActor` (`self.GetAvatarActorFromActorInfo`))
  (bind _ascharacter (cast `Character` (`BlackboardComponent.GetValueAsObject` (`AIBlueprintHelperLibrary.GetBlackboard` (`self.AvatarActor`)) (`self.Target Key Name`)))
    (:`then`
      (set `self.TargetLocation` (`Actor.K2_GetActorLocation` _ascharacter))
      (message `CombatInterface.UpdateMotionWarping` (`self.AvatarActor`) (`self.TargetLocation`))
      (bind (_montage _montagetag) (`self.GetAttackMontage`))
      (`AbilityTask_PlayMontageAndWait.CreatePlayMontageAndWaitProxy` "None" _montage
        (:`then`
          (`AbilityTask_WaitGameplayEvent.WaitGameplayEvent` _montagetag null true
            (:`EventReceived`
              (`self.SpawnProjectile` (`self.TargetLocation`)))))
        (:`OnCompleted`
          (`self.K2_EndAbility` :!label _label))
        (:`OnInterrupted`
          (goto _label))
        (:`OnCancelled`
          (goto _label))))
    (:`CastFailed`
      (`self.K2_EndAbility`))))

(fn `GetAttackMontage`
  (returns (Montage :type "AnimMontage Object Reference") (MontageTag :type "GameplayTag Structure"))
  (locals (AttackMontagesNumber :type Integer :default 0) (AttackMontages :type "TaggedMontage Structure"))
  (bind _returnvalue (message `CombatInterface.GetAttackMontages` (`self.AvatarActor`)))
  (bind _returnvalue_2 (`self.GetRandomTaggedMontageFromArray` _returnvalue))
  (bind _output_get (set `local.AttackMontages` _returnvalue_2))
  (bind (_montage _montagetag) (break `TaggedMontage` _output_get))
  (if (!= _montagetag (struct))
    (return _montage _montagetag)
    (else
      (`self.K2_EndAbility`))))