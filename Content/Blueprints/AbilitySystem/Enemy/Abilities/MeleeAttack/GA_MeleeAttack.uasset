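; Enemy melee attack ability that motion-warps toward the blackboard target and plays a random tagged attack montage.
; The montage's gameplay event stores the strike socket location and draws a debug sphere.
; A separate Sequence branch, not chained to that event, finds live actors around the stored location, damages non-friends and fires a melee GameplayCue at traced impact points.
; The ability ends when the montage completes, is interrupted or is cancelled.
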(event `self.K2_ActivateAbility`
  (bind _returnvalue (`self.GetAvatarActorFromActorInfo`))
  (`|ExecutionSequence`
    (:`then_0`
      (set `self.AvatarActor` _returnvalue)
      (bind _ascharacter (cast `Character` (`BlackboardComponent.GetValueAsObject` (`AIBlueprintHelperLibrary.GetBlackboard` _returnvalue) (`self.KeyForTarget`))))
      (message `CombatInterface.UpdateMotionWarping` (`self.AvatarActor`) (`Actor.K2_GetActorLocation` _ascharacter)))
    (:`then_1`
      (bind (_montage _montagetag _impact_sound _socket_location_tag) (`self.GetAttackMontage`))
      (set `self.CurrentMontageTag` _montagetag)
      (set `self.Impact Sound` _impact_sound)
      (`AbilityTask_PlayMontageAndWait.CreatePlayMontageAndWaitProxy` "None" _montage
        (:`then`
          (`AbilityAsync_WaitGameplayEvent.WaitGameplayEventToActor` (`self.AvatarActor`) (`self.CurrentMontageTag`) true
            (:`EventReceived`
              (bind _returnvalue_2 (message `CombatInterface.GetSocketLocation` (`self.AvatarActor`) _socket_location_tag))
              (bind _output_get (set `self.SocketLocation` _returnvalue_2))
              (`KismetSystemLibrary.DrawDebugSphere` _output_get (`self.Radius`) 12 (struct :`R` 1.0 :`G` 0.037902 :`A` 1.0) 2.0 1.0))))
        (:`OnCompleted`
          (`self.K2_EndAbility` :!label _label))
        (:`OnInterrupted`
          (goto _label))
        (:`OnCancelled`
          (goto _label))))
    (:`then_2`
      (bind _actorstoout (`UpFightAbilitySystemLibrary.GetLiveActorsFromRadius` (`self.AvatarActor`) (`|MakeArray` (`self.AvatarActor`)) (`self.Radius`) (`self.SocketLocation`)))
      (bind _output_get_2 (set `self.LiveActorsinRadius` _actorstoout))
      ; Пройдемся по тем кто в зоне удара, применим по ним эффект урона, далее трассировкой получим место удара и с помощью GC_MeleeImpact воспроизведем эффект удара и звук
      (for _array_element _output_get_2
        (set `self.TargetActor` _array_element)
        (if (not (`UpFightAbilitySystemLibrary.AreTheyFriends` (`self.AvatarActor`) (`self.TargetActor`)))
          (`UpFightAbilitySystemLibrary.UpFightApplyGameplayEffect` (`self.DamageEffect`) (`self.AvatarActor`) (`self.TargetActor`) (`self.DamageTypes`) (`KismetMathLibrary.Conv_IntToDouble` (`self.GetAbilityLevel`)))
          (bind _outhit (`KismetSystemLibrary.LineTraceSingle` (`self.SocketLocation`) (`Actor.K2_GetActorLocation` (`self.TargetActor`)) "TraceTypeQuery1" false (`|MakeArray` (`self.AvatarActor`)) "ForDuration" false (struct :`R` 1.0 :`A` 1.0) (struct :`G` 1.0 :`A` 1.0) 3.0))
          (`self.K2_ExecuteGameplayCueWithParams` (struct :`TagName` "GameplayCue.MeleeAttack") (`AbilitySystemBlueprintLibrary.MakeGameplayCueParameters` 0.0 0.0 (struct) (struct) (struct) (`BlueprintGameplayTagLibrary.MakeGameplayTagContainerFromTag` (`self.CurrentMontageTag`)) (struct) (`.ImpactPoint` (`GameplayStatics.BreakHitResult` _outhit)) (0.0 0.0 0.0) (`self.AvatarActor`) null (`self.TargetActor`))))))))

(fn `GetAttackMontage`
  (returns (Montage :type "AnimMontage Object Reference") (MontageTag :type "GameplayTag Structure") (`Impact Sound` :type "SoundBase Object Reference") (`Socket Location Tag` :type "GameplayTag Structure"))
  (locals (AttackMontages :type "TaggedMontage Structure") (AttackMontagesNumber :type Integer :default 0))
  (bind _returnvalue (message `CombatInterface.GetAttackMontages` (`self.AvatarActor`)))
  (bind _returnvalue_2 (`self.GetRandomTaggedMontageFromArray` _returnvalue))
  (bind _output_get (set `local.AttackMontages` _returnvalue_2))
  (bind (_montage _montagetag _socketlocationtag _impactsound) (break `TaggedMontage` _output_get))
  (if (!= _montagetag (struct))
    (return _montage _montagetag _impactsound _socketlocationtag)
    (else
      (`self.K2_EndAbility`))))