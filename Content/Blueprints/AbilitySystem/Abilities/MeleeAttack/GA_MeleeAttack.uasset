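; Melee attack gameplay ability for AI avatars that damages non-friendly live actors around a montage-tagged socket.
; It updates motion warping toward the blackboard target's location, then plays a random montage from the avatar's attack montages.
; The montage's gameplay event triggers one radius query at that socket, with a debug sphere, applying the damage effect at ability level.
; The ability ends when the montage completes, is interrupted or is cancelled.
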(event `self.K2_ActivateAbility`
  (bind _returnvalue (`self.GetAvatarActorFromActorInfo`))
  (set `self.AvatarActor` _returnvalue)
  (bind _ascharacter (cast `Character` (`BlackboardComponent.GetValueAsObject` (`AIBlueprintHelperLibrary.GetBlackboard` _returnvalue) (`self.KeyForTarget`))))
  (message `CombatInterface.UpdateMotionWarping` (`self.AvatarActor`) (`Actor.K2_GetActorLocation` _ascharacter))
  (bind (_montage _montagetag) (`self.GetAttackMontage`))
  (`AbilityTask_PlayMontageAndWait.CreatePlayMontageAndWaitProxy` "None" _montage
    (:`then`
      (`AbilityAsync_WaitGameplayEvent.WaitGameplayEventToActor` (`self.AvatarActor`) _montagetag true
        (:`EventReceived`
          (bind _returnvalue_2 (message `CombatInterface.GetSocketLocation` (`self.AvatarActor`) _montagetag))
          (`KismetSystemLibrary.DrawDebugSphere` _returnvalue_2 (`self.Radius`) 12 (struct :`R` 1.0 :`G` 0.037902 :`A` 1.0) 2.0 1.0)
          (bind _actorstoout (`UpFightAbilitySystemLibrary.GetLiveActorsFromRadius` (`self.AvatarActor`) (`|MakeArray` (`self.AvatarActor`)) (`self.Radius`) _returnvalue_2))
          (bind _output_get (set `self.LiveActorsinRadius` _actorstoout))
          (for _array_element _output_get
            (if (not (`UpFightAbilitySystemLibrary.AreTheyFriends` (`self.AvatarActor`) _array_element))
              (`UpFightAbilitySystemLibrary.UpFightApplyGameplayEffect` (`self.DamageEffect`) (`self.AvatarActor`) _array_element (`self.DamageTypes`) (`KismetMathLibrary.Conv_IntToDouble` (`self.GetAbilityLevel`))))))))
    (:`OnCompleted`
      (`self.K2_EndAbility` :!label _label))
    (:`OnInterrupted`
      (goto _label))
    (:`OnCancelled`
      (goto _label))))

(fn `GetAttackMontage`
  (returns (Montage :type "AnimMontage Object Reference") (MontageTag :type "GameplayTag Structure"))
  (locals (AttackMontages :type "TaggedMontage Structure") (AttackMontagesNumber :type Integer :default 0))
  (bind _returnvalue (message `CombatInterface.GetAttackMontages` (`self.AvatarActor`)))
  (set `local.AttackMontagesNumber` (`KismetArrayLibrary.Array_Length` _returnvalue))
  (if (> (`local.AttackMontagesNumber`) 0)
    (bind _output_get (set `local.AttackMontages` (`|GetArrayItem` _returnvalue (`KismetMathLibrary.RandomIntegerInRange` 0 (- (`local.AttackMontagesNumber`) 1)))))
    (bind (_montage _montagetag) (break `TaggedMontage` _output_get))
    (return _montage _montagetag)
    (else
      (`self.K2_EndAbility`))))